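; Base player character that provides camera-relative movement, a spring-arm camera and visual feedback for skills and invisibility.
; Move inputs follow control yaw, and a vision toggle switches the spring arm between a near and far length.
; Helpers show one of three skill range decals and swap the mesh between hiding, invisible and cached default materials.
; Mine-step events are forwarded to the owning GameplayPC controller.
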(event Custom|FOOL_charStepOnMine
  (params (ownerPC :type Gameplay%20PC%20Object%20Reference) (mine :type M%20Fool%20Mine%20Object%20Reference))
  (bind _asgameplay_pc (Utilities|Casting|CastToGameplayPC (Pawn|GetController)))
  (Default|FOOLSteponMine _asgameplay_pc ownerPC mine))

(event Custom|toggleVision
  (params (isLarger :type Boolean))
  (if isLarger
    (Variables|/Script/Engine.SpringArmComponent|SetTargetArmLength (Variables|Default|GetSpringArm1) 1.2e+03)
    (else
      (Variables|/Script/Engine.SpringArmComponent|SetTargetArmLength (Variables|Default|GetSpringArm1) 8e+02))))

(event EventBeginPlay
  (Components|Activation|Activate (Variables|Default|GetCamera1) false))

(event Input|AxisEvents|InputAxisMoveForward
  (params (AxisValue :type Float%20%28single-precision%29))
  (Pawn|Input|AddMovementInput (Math|Vector|GetForwardVector (Math|Rotator|MakeRotator 0.0 0.0 (.Yaw (Math|Rotator|BreakRotator (Pawn|GetControlRotation :!class /Script/Engine.Pawn))))) AxisValue false))

(event Input|AxisEvents|InputAxisMoveRight
  (params (AxisValue :type Float%20%28single-precision%29))
  (Pawn|Input|AddMovementInput (Math|Vector|GetRightVector (Math|Rotator|MakeRotator 0.0 0.0 (.Yaw (Math|Rotator|BreakRotator (Pawn|GetControlRotation :!class /Script/Engine.Pawn))))) AxisValue false))

(fn ConstructionScript
  (Variables|Default|SetdefaultMaterial (Utilities|Array|Get(acopy) (Rendering|Material|GetMaterials (Variables|Character|GetMesh)))))

(fn ToggleSkillSelectRing
  (params (turnOn :type Boolean) (toggleWhich :type Integer))
  (switch int toggleWhich
    (:Default
      (Development|PrintString "Cannot determine which decal to toggle"))
    (:0
      (LocalVariables|SettoggleDecalTarget (Variables|Default|GetSelectRing300))
      (if turnOn :!label _label
        (Rendering|SetVisibility (LocalVariables|GettoggleDecalTarget) true false)
        (else
          (Rendering|SetVisibility (LocalVariables|GettoggleDecalTarget) false false))))
    (:1
      (LocalVariables|SettoggleDecalTarget (Variables|Default|GetSelectRing500))
      (goto _label))
    (:2
      (LocalVariables|SettoggleDecalTarget (Variables|Default|GetSelectRing200))
      (goto _label))))

(fn UpdateOnlyPlayerCanSee
  (params (isGivenInvisibility :type Boolean) (isHiding :type Boolean))
  (if isGivenInvisibility
    (if isHiding
      (Rendering|Material|SetMaterial (Variables|Character|GetMesh) 0 "/Game/Materials/Decals/Invisible_Green.Invisible_Green")
      (else
        (Rendering|Material|SetMaterial (Variables|Character|GetMesh) 0 "/Game/Materials/Decals/Invisible_Yellow.Invisible_Yellow")))
    (else
      (Rendering|Material|SetMaterial (Variables|Character|GetMesh) 0 (Variables|Default|GetdefaultMaterial)))))