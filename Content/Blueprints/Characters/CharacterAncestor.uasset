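; CharacterAncestor is a base character Blueprint that handles being clicked as a target for the player's kill ability.
; On click, it gets player 0's GameplayPC and rejects self-targeting with a player-only notification.
; Otherwise it passes itself to ProcessKillRequest if the kill ability is selected, or prompts the player to select a skill first.
; BeginPlay, overlap and Tick are empty, and an UpdateTargeting call is left unwired.
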(event EventBeginPlay)

(event Collision|EventActorBeginOverlap
  (params (OtherActor :type Actor%20Object%20Reference)))

(event EventTick
  (params (DeltaSeconds :type Float%20%28single-precision%29)))

(event MouseInput|EventActorOnClicked
  (params (ButtonPressed :type Key%20Structure))
  ;[1 1 1] onClick event, check whether clicking character selects kill or any skill.
  (bind _asgameplay_pc_new (Utilities|Casting|CastToGameplayPC (Game|GetPlayerController 0)))
  (if (== (Pawn|GetControlledPawn _asgameplay_pc_new) self)
    (Default|PrintNewNotification _asgameplay_pc_new "Can't target yourself" true)
    (elif (Variables|/Game/Blueprints/Gameplay/GameplayPC.GameplayPC_C|GetisSelectKillAbility _asgameplay_pc_new)
      (Default|ProcessKillRequest _asgameplay_pc_new self)
      (else
        (Default|PrintNewNotification _asgameplay_pc_new "Select a Skill first" true)))))

(fn ConstructionScript)