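; InfoPC is a player controller that handles the info screens and the exit from a session.
; Escape toggles the BackForInfo menu along with the mouse cursor, and Tab shows or hides the Introduction widget, each through a FlipFlop.
; Showing either widget creates a fresh instance.
; EndPlay destroys the session, and Kicked opens MainMenu before destroying it.
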(event Custom|SetupIntroduction
  ;[1 1 1] Setup intro duction widget
  (Widget|RemovefromParent (Variables|Default|GetIntroductionWB))
  (bind _returnvalue (UserInterface|CreateWidget "/Game/UI/Info/Introduction.Introduction_C"))
  (bind _output_get (Variables|Default|SetIntroductionWB _returnvalue))
  (UserInterface|Viewport|AddtoViewport _output_get 0))

(event Custom|Kicked
  ;[1 1 1] Back to main
  (Game|OpenLevel(byName) "MainMenu")
  (|DestroySession self))

(event EventEndPlay
  (params (EndPlayReason :type EEndPlayReason%20Enum :default "Destroyed"))
  ;[1 1 1] Back to main
  (|DestroySession self))

(event Input|KeyboardEvents|Escape
  (params (Key :type Key%20Structure :default "None"))
  ;[1 1 1] Press esC to exit
  (:Pressed
    (Utilities|FlowControl|FlipFlop
      (:A
        (Variables|Default|SetbShowMouseCursor true)
        (bind _returnvalue (UserInterface|CreateWidget "/Game/UI/Info/BackForInfo.BackForInfo_C" (Game|GetPlayerController 0)))
        (Variables|Default|SetBackMenuWB _returnvalue)
        (UserInterface|Viewport|AddtoViewport (Variables|Default|GetBackMenuWB) 0))
      (:B
        (Variables|Default|SetbShowMouseCursor false)
        (Widget|RemovefromParent (Variables|Default|GetBackMenuWB))))))

(event Input|KeyboardEvents|Tab
  (params (Key :type Key%20Structure :default "None"))
  ;[1 1 1] Press tab to show/hide
  (:Pressed
    (Utilities|FlowControl|FlipFlop
      (:A
        (CallFunction|SetupIntroduction))
      (:B
        (Widget|RemovefromParent (Variables|Default|GetIntroductionWB))))))

(fn ConstructionScript)