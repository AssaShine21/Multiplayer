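; Vector math helper functions for AI movement, centered on a Particle Swarm Optimization (PSO) velocity update.
; The PSO step adds randomly weighted pulls toward personal-best and global-best locations to the current velocity, then clamps its length to a maximum.
; Other helpers give random 3D or flattened 2D velocities at a given magnitude.
; Despite its 2D name, the PSO function leaves Z intact.
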(fn GetVelocityComponent
  (params (current :type Vector) (target :type Vector) (magnitude :type Float%20%28single-precision%29))
  (return (* (- target current) magnitude)))

(fn GetRandomVelocity3D
  (params (magnitude :type Float%20%28single-precision%29))
  (return (* (Math|Random|RandomUnitVector) magnitude)))

(fn GetRandomVelocity2D
  (params (magnitude :type Float%20%28single-precision%29))
  (return (* (Class|KismetMathLibrary|VectorNormal2D (Math|Random|RandomUnitVector) 0.0001) magnitude)))

(fn GetPSONewVelocity2D
  (params (pBestLocation :type Vector) (gBestLocation :type Vector) (currentLocation :type Vector) (currentVelocity :type Vector) (pCoeffi :type Float%20%28single-precision%29) (gCoeffi :type Float%20%28single-precision%29) (maxVelocityMagnitude :type Float%20%28single-precision%29))
  ;[1 1 1] PSO: v_i' = v_i + c_1 * rand() * (pbest - x_i) + c_2 * rand() * (gbest - x_i)
  (bind _res (CallFunction|GetVelocityComponent currentLocation pBestLocation (Math|Random|RandomFloatinRange 0.0 pCoeffi)))
  (bind _res_2 (CallFunction|GetVelocityComponent currentLocation gBestLocation (Math|Random|RandomFloatinRange 0.0 gCoeffi)))
  (bind _checkedvelocity (CallFunction|CheckMaxVelocity (+ currentVelocity _res _res_2) maxVelocityMagnitude))
  (return _checkedvelocity))

(fn CheckMaxVelocity
  (params (velocity :type Vector) (maxVelocityMagnitude :type Float%20%28single-precision%29))
  (if (<= (Math|Vector|VectorLength velocity) maxVelocityMagnitude)
    (return velocity)
    (else
      (return (* (Math|Vector|Normalize velocity) maxVelocityMagnitude)))))