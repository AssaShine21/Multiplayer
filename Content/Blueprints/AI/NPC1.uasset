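; NPC1 is an AI character, given one of four random skeletal meshes at spawn, that moves under particle swarm pathfinding.
; On BeginPlay it finds the ParticleSwarmPath actor and takes an initial velocity from it.
; While CanMove is set, Tick decomposes velocity into target points, issues AIMoveTo through random delays, then requests an updated velocity from the path finder.
; Some disconnected movement experiments, including a random trail, remain unused.
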(event EventTick
  (params (DeltaSeconds :type Float%20%28single-precision%29))
  (bind _self self)
  (if (Variables|Default|GetcanMove)
    (bind _res (CallFunction|SimpleDecompose (Variables|Default|Getvelocity)))
    (bind _res_2 (CallFunction|GetTargetVectorSequences _res (Transformation|GetActorLocation)))
    (for _array_element _res_2
      (Utilities|FlowControl|Delay (Math|Random|RandomFloatinRange 0.0 3.0))
      (AI|AIMoveTo self _array_element 0 5.0 true))
    ;[1 1 1] Update velocity
    (bind _newvelocity (Class|PathFinderInterface|UpdateVelocity(Message) (Variables|Default|GetpathFinder) _self (Transformation|GetActorLocation _self) (Variables|Default|Getvelocity)))
    (Variables|Default|Setvelocity _newvelocity)))

(event EventBeginPlay
  (bind _mesh (Variables|Character|GetMesh))
  ;[1 1 1] Get reference to path finder control and set initial velocity
  (bind _returnvalue (Actor|GetActorOfClass "/Game/Blueprints/AI/ParticleSwarmPath.ParticleSwarmPath_C"))
  (CallFunction|Initialise _returnvalue)
  (switch int (Math|Random|RandomInteger 4)
    (:Default
      (Class|SkinnedMeshComponent|SetSkeletalMesh _mesh "/Game/InfinityBladeWarriors/Character/CompleteCharacters/SK_CharM_Forge.SK_CharM_Forge" true))
    (:0
      (Class|SkinnedMeshComponent|SetSkeletalMesh _mesh "/Game/InfinityBladeWarriors/Character/CompleteCharacters/SK_CharM_Barbarous.SK_CharM_Barbarous" true))
    (:1
      (Class|SkinnedMeshComponent|SetSkeletalMesh _mesh "/Game/InfinityBladeWarriors/Character/CompleteCharacters/SK_CharM_Robo.SK_CharM_Robo" true))
    (:2
      (Class|SkinnedMeshComponent|SetSkeletalMesh _mesh "/Game/InfinityBladeWarriors/Character/CompleteCharacters/SK_CharM_FrostGiant.SK_CharM_FrostGiant" true))))

(fn ConstructionScript)

(fn Initialise
  (params (pathFinder :type Particle%20Swarm%20Path%20Object%20Reference))
  (bind _output_get (Variables|Default|SetpathFinder pathFinder))
  (bind _velocity (Class|PathFinderInterface|GetInitialVelocity(Message) _output_get))
  (Variables|Default|Setvelocity _velocity))

(fn UpdateCanMove
  (params (newCanMove :type Boolean))
  (Variables|Default|SetcanMove newCanMove))