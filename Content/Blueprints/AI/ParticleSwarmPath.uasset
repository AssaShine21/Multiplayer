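; Path finder actor that creates five NPCs at BeginPlay and guides them with 2D particle swarm optimisation.
; Each Tick compares every NPC1 location against its personal best and the global best, minimising a placeholder cost function of X and Y.
; UpdateVelocity combines both bests into a new velocity, falling back to random for unknown NPCs.
; GetInitialVelocity supplies random starting velocities.
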(event Collision|EventActorBeginOverlap
  (params (OtherActor :type Actor%20Object%20Reference)))

(event EventBeginPlay
  ;[1 1 1] set path finder hidden and initialise NPC
  (Rendering|SetActorHiddenInGame false)
  (CallFunction|CreateNPC 5)
  ;[1 1 1] Set Reference to all NPCs, performed only once.
  (bind _outactors (Actor|GetAllActorsOfClass "/Game/Blueprints/AI/NPC1.NPC1_C"))
  (Variables|Default|Setnpcs _outactors)
  ;[1 1 1] Set Parameters
  (Variables|Default|SetpCoeffi 0.5)
  (Variables|Default|SetgCoeffi 0.8)
  (Variables|Default|SetmaxVelocityMagnitude 5e+02))

(event EventTick
  (params (DeltaSeconds :type Float%20%28single-precision%29))
  ;[1 1 1] Update pBest for each NPC and gBest for all
  (for (_array_element _array_index) (Variables|Default|Getnpcs)
    (bind _isupdated (CallFunction|UpdatePBest _array_index (Transformation|GetActorLocation _array_element)))
    (if _isupdated
      (CallFunction|UpdateGBest (Transformation|GetActorLocation _array_element)))))

(fn ConstructionScript)

(fn UpdatePBest
  (params (npcId :type Integer) (npcLocation :type Vector))
  (bind _pbests (Variables|Default|GetpBests))
  (bind _output (Utilities|Array|Get(acopy) _pbests npcId))
  (if (Math|Vector|Equal(Vector) _output "0, 0, 0" 0.0001)
    _
    (else
      (bind _res (CallFunction|HiddenFunction npcLocation))
      (bind _res_2 (CallFunction|HiddenFunction _output))
      (if (<= _res _res_2)
        _
        (else
          (return false)))))
  (Utilities|Array|SetArrayElem (Variables|Default|GetpBests) npcId npcLocation)
  (return true))

(fn UpdateGBest
  (params (npcLocation :type Vector))
  (if (Math|Vector|Equal(Vector) (Variables|Default|GetgBest) "0, 0, 0" 0.0001)
    _
    (else
      (bind _res (CallFunction|HiddenFunction npcLocation))
      (bind _res_2 (CallFunction|HiddenFunction (Variables|Default|GetgBest)))
      (if (<= _res _res_2)
        _
        (else
          (return false)))))
  (Variables|Default|SetgBest npcLocation)
  (return true))

(fn HiddenFunction
  (params (currentLocation :type Vector))
  (bind (_x _y) (Math|Vector|BreakVector currentLocation))
  ;[1 1 1] A simple function to minimise value, can change later according to gameplay
  (return (|((pow((x+100),2))+(pow(y,4))) _x _y)))

(fn GetInitialVelocity
  (bind _res (CallFunction|GetRandomVelocity2D (Variables|Default|GetmaxVelocityMagnitude)))
  (return _res))

(fn UpdateVelocity
  (params (npc :type NPC1%20Object%20Reference) (currentLocation :type Vector :default "0, 0, 0") (currentVelocity :type Vector :default "0, 0, 0"))
  (for (_array_element _array_index) (Variables|Default|Getnpcs)
    (if (== _array_element npc)
      (bind _newvelocity (CallFunction|GetPSONewVelocity2D (Utilities|Array|Get(acopy) (Variables|Default|GetpBests) _array_index) (Variables|Default|GetgBest) currentLocation currentVelocity (Variables|Default|GetpCoeffi) (Variables|Default|GetgCoeffi) (Variables|Default|GetmaxVelocityMagnitude)))
      (return _newvelocity true)))
  (bind _res (CallFunction|GetRandomVelocity2D (Variables|Default|GetmaxVelocityMagnitude)))
  (return _res false))