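; NPC spawner actor that populates the level with NPC1 AI pawns at random navigable points around a fixed origin.
; BeginPlay spawns an initial batch, and Tick adds one per frame while the world count is below MaxCount; its trailing Delay gates nothing.
; It caches spawned NPCs, syncs that list to PSOManager and broadcasts the can-move flag.
; DeleteNPC unregisters and freezes an NPC without destroying it.
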(event EventBeginPlay
  (for _index (range 1 (Variables|Default|GetinitialCount))
    (bind _randomlocation (Class|NavigationSystemV1|GetRandomLocationinNavigableRadius (Math|Conversions|ToVector(Float) (Utilities|Struct|MakeIntVector -800 -2 170)) 3e+03 0 0))
    (bind _returnvalue (AI|SpawnAIFromClass "/Game/Blueprints/AI/NPC1.NPC1_C" 0 _randomlocation "0, 0, 0" false 0))
    (bind _asnpc1 (Utilities|Casting|CastToNPC1 _returnvalue))
    (Default|UpdateCanMove _asnpc1 (Variables|Default|GetnewNPC_CanMove))
    (Utilities|Array|Add (Variables|Default|GetallNPCs) _asnpc1)
    (Default|UpdateAllNPCs (Variables|Default|GetPSO_Manager) (Variables|Default|GetallNPCs))))

(event Collision|EventActorBeginOverlap
  (params (OtherActor :type Actor%20Object%20Reference)))

(event EventTick
  (params (DeltaSeconds :type Float%20%28single-precision%29))
  (bind _outactors (Actor|GetAllActorsOfClass "/Game/Blueprints/AI/NPC1.NPC1_C"))
  (if (< (Utilities|Array|Length _outactors) (Variables|Default|GetmaxCount))
    (bind _randomlocation (Class|NavigationSystemV1|GetRandomLocationinNavigableRadius (Math|Conversions|ToVector(Float) (Utilities|Struct|MakeIntVector -800 -2 170)) 3e+03 0 0))
    (bind _returnvalue (AI|SpawnAIFromClass "/Game/Blueprints/AI/NPC1.NPC1_C" 0 _randomlocation "0, 0, 0" false 0))
    (bind _asnpc1 (Utilities|Casting|CastToNPC1 _returnvalue))
    (Default|UpdateCanMove _asnpc1 (Variables|Default|GetnewNPC_CanMove))
    (Utilities|Array|Add (Variables|Default|GetallNPCs) _asnpc1)
    (Default|UpdateAllNPCs (Variables|Default|GetPSO_Manager) (Variables|Default|GetallNPCs)))
  (Utilities|FlowControl|Delay 1e+01))

(fn ConstructionScript)

(fn GetAllNPCs
  ;[1 1 1] Avoid "get all actors by class" to save time
  (return (Variables|Default|GetallNPCs)))

(fn UpdateCanMoves
  (params (newCanMoves :type Boolean))
  (Variables|Default|SetnewNPC_CanMove newCanMoves)
  (for _array_element (Variables|Default|GetallNPCs)
    (Default|UpdateCanMove _array_element newCanMoves)))

(fn DeleteNPC
  (params (target :type NPC1%20Object%20Reference))
  (Utilities|Array|RemoveItem (Variables|Default|GetallNPCs) target)
  (Default|RemoveNPC (Variables|Default|GetPSO_Manager) target)
  (Default|FreezeNPC target))