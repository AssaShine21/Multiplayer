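; NPC population manager that spawns an initial crowd at random navigable points around a fixed origin, then tops it up toward a maximum through a delayed Tick.
; Each spawn picks one of the character classes by weighted random draw, heavily favoring those flagged as selected.
; It caches all NPCs to avoid actor searches, syncs them with PSOManager, broadcasts movement permission, and freezes NPCs it removes.
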(event Custom|updateCharsSelected
  (params (newCharsArray :type Array%20of%20Booleans))
  (Variables|Default|SetisCharSelectedArray newCharsArray)
  (CallFunction|InitMeshSampling))

(event EventBeginPlay
  (CallFunction|InitMeshSampling)
  (for _index (range 1 (Variables|Default|GetinitialCount))
    (bind _randomlocation (Class|NavigationSystemV1|GetRandomLocationinNavigableRadius (Math|Conversions|ToVector(Float) (Utilities|Struct|MakeIntVector -800 -2 170)) 3e+03 0 0))
    (bind _resclass (CallFunction|GetRandomClass))
    (bind _returnvalue (AI|SpawnAIFromClass _resclass 0 _randomlocation "0, 0, 0" false 0))
    (bind _asnpc1 (Utilities|Casting|CastToNPC1 _returnvalue))
    (Default|UpdateCanMove _asnpc1 (Variables|Default|GetnewNPC_CanMove))
    (Utilities|Array|Add (Variables|Default|GetallNPCs) _asnpc1)
    (Default|UpdateAllNPCs (Variables|Default|GetPSO_Manager) (Variables|Default|GetallNPCs))))

(event EventTick
  (params (DeltaSeconds :type Float%20%28single-precision%29))
  (Utilities|FlowControl|Delay 2.0)
  (if (< (Utilities|Array|Length (Variables|Default|GetallNPCs)) (Variables|Default|GetmaxCount))
    (bind _randomlocation (Class|NavigationSystemV1|GetRandomLocationinNavigableRadius (Math|Conversions|ToVector(Float) (Utilities|Struct|MakeIntVector -800 -2 170)) 3e+03 0 0))
    (bind _resclass (CallFunction|GetRandomClass))
    (bind _returnvalue (AI|SpawnAIFromClass _resclass 0 _randomlocation "0, 0, 0" false 0))
    (bind _asnpc1 (Utilities|Casting|CastToNPC1 _returnvalue))
    (Default|UpdateCanMove _asnpc1 (Variables|Default|GetnewNPC_CanMove))
    (Utilities|Array|Add (Variables|Default|GetallNPCs) _asnpc1)
    (Default|UpdateAllNPCs (Variables|Default|GetPSO_Manager) (Variables|Default|GetallNPCs))))

(fn ConstructionScript)

(fn GetAllNPCs
  ;[1 1 1] Avoid "get all actors by class" to save time
  (return (Variables|Default|GetallNPCs)))

(fn UpdateCanMoves
  (params (newCanMoves :type Boolean))
  (Variables|Default|SetnewNPC_CanMove newCanMoves)
  (for _array_element (Variables|Default|GetallNPCs)
    (Default|UpdateCanMove _array_element newCanMoves)))

(fn DeleteNPC
  (params (target :type NPC1%20Object%20Reference))
  (Utilities|Array|RemoveItem (Variables|Default|GetallNPCs) target)
  (Default|RemoveNPC (Variables|Default|GetPSO_Manager) target)
  (Default|FreezeNPC target))

(fn InitMeshSampling
  (Variables|Default|SetselectedToUnselectedRatio 9)
  (Variables|Default|SetselectionTotalPool 0)
  (for _array_element (Variables|Default|GetisCharSelectedArray)
    (if _array_element
      (Variables|Default|SetselectionTotalPool (+ (Variables|Default|GetselectionTotalPool) (Variables|Default|GetselectedToUnselectedRatio)))
      (else
        (Variables|Default|SetselectionTotalPool (+ (Variables|Default|GetselectionTotalPool) 1))))))

(fn GetRandomClass
  (LocalVariables|Setremaining (Math|Random|RandomIntegerinRange 1 (Variables|Default|GetselectionTotalPool)))
  (for (_array_element _array_index) (Variables|Default|GetisCharSelectedArray)
    (if _array_element
      (LocalVariables|Setremaining (- (LocalVariables|Getremaining) (Variables|Default|GetselectedToUnselectedRatio)))
      (else
        (LocalVariables|Setremaining (- (LocalVariables|Getremaining) 1))))
    (if (<= (LocalVariables|Getremaining) 0)
      (bind _resclass (CallFunction|GetClassfromId _array_index))
      (return _resclass))))

(fn GetMeshfromId
  (params (id :type Integer))
  (switch int id
    (:Default
      (return "/Game/Character/Vampire/vampire.vampire"))
    (:0
      (return "/Game/Character/Archer/archer.archer"))
    (:1
      (return "/Game/Character/barbarous/Ske_mesh_barbarous.Ske_mesh_barbarous"))
    (:2
      (return "/Game/Character/Fool/fool.fool"))
    (:3
      (return "/Game/Character/Gambler/gambler.gambler"))
    (:4
      (return "/Game/Character/Mage/mage.mage"))
    (:5
      (return "/Game/Character/Policeman/policeman.policeman"))
    (:6
      (return "/Game/Character/PuppetMaster/puppet.puppet"))))

(fn GetClassfromId
  (params (id :type Integer))
  (switch int id
    (:Default
      (return "/Game/Blueprints/AI/NPC_Children/NPC_VAMP.NPC_VAMP_C"))
    (:0
      (return "/Game/Blueprints/AI/NPC_Children/NPC_ARCH.NPC_ARCH_C"))
    (:1
      (return "/Game/Blueprints/AI/NPC_Children/NPC_BARB.NPC_BARB_C"))
    (:2
      (return "/Game/Blueprints/AI/NPC_Children/NPC_FOOL.NPC_FOOL_C"))
    (:3
      (return "/Game/Blueprints/AI/NPC_Children/NPC_GAMB.NPC_GAMB_C"))
    (:4
      (return "/Game/Blueprints/AI/NPC_Children/NPC_MAGE.NPC_MAGE_C"))
    (:5
      (return "/Game/Blueprints/AI/NPC_Children/NPC_POLI.NPC_POLI_C"))
    (:6
      (return "/Game/Blueprints/AI/NPC_Children/NPC_PUPP.NPC_PUPP_C"))))