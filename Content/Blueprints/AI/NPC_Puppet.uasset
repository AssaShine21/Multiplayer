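; NPC_Puppet is a short-lived wandering NPC that sets its puppet mesh at construction and destroys itself 15 seconds after BeginPlay.
; Each Tick takes the offset between its location and a random reachable nearby point, decomposes it, and turns it into target positions from its location.
; A loop over those targets feeds AIMoveTo through a random Delay, with both latent nodes inside the per-frame loop.
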(event Custom|destroyThisPuppet
  (Actor|DestroyActor))

(event EventTick
  (params (DeltaSeconds :type Float%20%28single-precision%29))
  (bind _returnvalue (Transformation|GetActorLocation))
  (bind _res (CallFunction|SimpleDecompose (- _returnvalue (.RandomLocation (AI|Navigation|GetRandomReachablePointinRadius _returnvalue 5e+02 0 0)))))
  (bind _res_2 (CallFunction|GetTargetVectorSequences _res (Transformation|GetActorLocation)))
  (for _array_element _res_2
    (Utilities|FlowControl|Delay (Math|Random|RandomFloatinRange 0.0 3.0))
    (AI|AIMoveTo self _array_element 0 5.0 true)))

(event EventBeginPlay
  (Utilities|Time|SetTimerbyEvent (delegate Custom|destroyThisPuppet) 15.0))

(fn ConstructionScript
  (Class|SkinnedMeshComponent|SetSkeletalMesh (Variables|Character|GetMesh) "/Game/Character/PuppetMaster/puppet.puppet" true))