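; Gameplay game state that stores each player's in-game info: skill availability, character enum, gambling multiplier and who is investigating them.
; Entries live in the EveryoneInGameInfo struct array, found by a linear search on PlayerController.
; Each update function rewrites one field of the matching entry and copies the rest.
; Missing players get a new default entry, except in the investigation update, which only prints an error.
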(event EventBeginPlay)

(event EventTick
  (params (DeltaSeconds :type Float%20%28single-precision%29)))

(fn ConstructionScript)

(fn GetinGameInfoStructbyPC
  (params (player :type Gameplay%20PC%20Object%20Reference))
  (for (_array_element _array_index) (Variables|Default|GetEveryoneInGameInfo)
    (if (== (.playercontroller _array_element) player)
      (return true _array_index (Utilities|Array|Get(acopy) (Variables|Default|GetEveryoneInGameInfo) _array_index))))
  (return false 0 ""))

(fn UpdatePlayerSkillsAvail
  (params (player :type Gameplay%20PC%20Object%20Reference) (skillsAvail :type Array%20of%20Booleans))
  (LocalVariables|SetcurrPlayer player)
  (LocalVariables|SetcurrSkillsAvail skillsAvail)
  (bind (_found _targetindex _resgamestate) (CallFunction|GetinGameInfoStructbyPC (LocalVariables|GetcurrPlayer)))
  (if _found
    (bind _output_get (LocalVariables|SettargetStruct _resgamestate))
    (Utilities|Array|SetArrayElem (Variables|Default|GetEveryoneInGameInfo) _targetindex (Utilities|Struct|MakeinGameStruct (.playercontroller _output_get) (LocalVariables|GetcurrSkillsAvail) (.charenum _output_get) (.gamblingmultiplier _output_get) (.poliinvestigatedby _output_get)))
    (else
      (Utilities|Array|Add (Variables|Default|GetEveryoneInGameInfo) (Utilities|Struct|MakeinGameStruct (LocalVariables|GetcurrPlayer) (LocalVariables|GetcurrSkillsAvail) "NewEnumerator0" 1.0 0)))))

(fn UpdatePlayerCharEnum
  (params (player :type Gameplay%20PC%20Object%20Reference) (charEnum :type CharClassEnum%20Enum :default "NewEnumerator0"))
  (LocalVariables|SetcurrPlayer player)
  (LocalVariables|SetcurrCharEnum charEnum)
  (bind (_found _targetindex _resgamestate) (CallFunction|GetinGameInfoStructbyPC (LocalVariables|GetcurrPlayer)))
  (if _found
    (bind _output_get (LocalVariables|SettargetStruct _resgamestate))
    (Utilities|Array|SetArrayElem (Variables|Default|GetEveryoneInGameInfo) _targetindex (Utilities|Struct|MakeinGameStruct (.playercontroller _output_get) (.skillsavailability _output_get) (LocalVariables|GetcurrCharEnum) (.gamblingmultiplier _output_get) (.poliinvestigatedby _output_get)))
    (else
      (Utilities|Array|Add (Variables|Default|GetEveryoneInGameInfo) (Utilities|Struct|MakeinGameStruct (LocalVariables|GetcurrPlayer) "(True,True,True,True)" (LocalVariables|GetcurrCharEnum) 1.0 0)))))

(fn UpdatePlayerGambling
  (params (player :type Gameplay%20PC%20Object%20Reference) (gamblingMultiplier :type Float%20%28single-precision%29))
  (LocalVariables|SetcurrPlayer player)
  (LocalVariables|SetcurrGambling gamblingMultiplier)
  (bind (_found _targetindex _resgamestate) (CallFunction|GetinGameInfoStructbyPC (LocalVariables|GetcurrPlayer)))
  (if _found
    (bind _output_get (LocalVariables|SettargetStruct _resgamestate))
    (Utilities|Array|SetArrayElem (Variables|Default|GetEveryoneInGameInfo) _targetindex (Utilities|Struct|MakeinGameStruct (.playercontroller _output_get) (.skillsavailability _output_get) (.charenum _output_get) (LocalVariables|GetcurrGambling) (.poliinvestigatedby _output_get)))
    (else
      (Utilities|Array|Add (Variables|Default|GetEveryoneInGameInfo) (Utilities|Struct|MakeinGameStruct (LocalVariables|GetcurrPlayer) "(True,True,True,True)" "NewEnumerator0" (LocalVariables|GetcurrGambling) 0)))))

(fn UpdatePlayerInvestigatedby
  (params (player :type Gameplay%20PC%20Object%20Reference) (isInvestigated :type Boolean) (investigator :type Gameplay%20PC%20Object%20Reference))
  (LocalVariables|SetcurrPlayer player)
  (if isInvestigated
    (LocalVariables|SetcurrInvestigator investigator))
  (bind (_found _targetindex _resgamestate) (CallFunction|GetinGameInfoStructbyPC (LocalVariables|GetcurrPlayer)))
  (if _found
    (bind _output_get (LocalVariables|SettargetStruct _resgamestate))
    (Utilities|Array|SetArrayElem (Variables|Default|GetEveryoneInGameInfo) _targetindex (Utilities|Struct|MakeinGameStruct (.playercontroller _output_get) (.skillsavailability _output_get) (.charenum _output_get) (.gamblingmultiplier _output_get) (LocalVariables|GetcurrInvestigator)))
    (else
      (Development|PrintString "Cannot find target to investigate in GS"))))